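; Player character that is a rubbish heap, with axis-driven movement and look, and a HUD created at BeginPlay.
; Tick binds MeshChange to the game mode's TrashCollected event, swapping between three pile meshes by PendingScore and easing the spring arm length to match.
; RemoveTime briefly flashes a damaged material and deducts ten seconds from the game mode's timer.
; Buoyancy animation and trace-based force logic exist but never run.
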(event `Damage`
  (bind _trashheap (`self.TrashHeap`))
  (`PrimitiveComponent.SetMaterial` _trashheap 0 "/Game/Assets/Materials/MI_RubbishHeapDamaged.MI_RubbishHeapDamaged")
  (`KismetSystemLibrary.Delay` 0.1)
  (`PrimitiveComponent.SetMaterial` _trashheap 0 "/Game/Assets/Materials/M_RubbishHeap.M_RubbishHeap"))

(event `self.ReceiveBeginPlay`
  (`|ExecutionSequence`
    (:`then_0`
      (bind _asgm_default (cast `/Game/Blueprints/Character/GM_Default` (`GameplayStatics.GetGameMode`)))
      (set `self.GMRef` _asgm_default))
    (:`then_1`
      (bind _returnvalue (`|CreateWidget` "/Game/Blueprints/Widgets/UI/WBP_HUD.WBP_HUD_C" (`GameplayStatics.GetPlayerController` 0)))
      (bind _output_get (set `self.HUDRef` _returnvalue))
      (`UserWidget.AddToViewport` _output_get 0))))

(event `InputAxis|MoveForward`
  (params (AxisValue :type "Float (single-precision)"))
  ;[1 0.02344 0] Movement
  (`self.AddMovementInput` (`self.GetActorForwardVector`) AxisValue))

(event `InputAxis|LookUp`
  (params (AxisValue :type "Float (single-precision)"))
  ;[1 0.02344 0] Movement
  (`self.AddControllerPitchInput` AxisValue))

(event `InputAxis|LookRight`
  (params (AxisValue :type "Float (single-precision)"))
  ;[1 0.02344 0] Movement
  (`self.AddControllerYawInput` AxisValue))

(event `InputAxis|MoveRight`
  (params (AxisValue :type "Float (single-precision)"))
  ;[1 0.02344 0] Movement
  (`self.AddMovementInput` (`self.GetActorRightVector`) AxisValue))

(event `self.ReceiveTick`
  (params (DeltaSeconds :type "Float (single-precision)"))
  (add `/Game/Blueprints/Character/GM_Default.TrashCollected` (`self.GMRef`) (delegate `MeshChange`)))

(event `MeshChange`
  (bind _springarm (`self.SpringArm`))
  (bind _meshsize (`self.MeshSize`))
  (bind _pendingscore (`/Game/Blueprints/Character/GM_Default.PendingScore` (`self.GMRef`)))
  (if (<= _pendingscore (`self.SmallMeshValue`))
    (set `self.MeshSize` 0)
    (`StaticMeshComponent.SetStaticMesh` (`self.TrashHeap`) (select `int` _meshsize :`0` "/Game/Assets/Meshes/SM_RubbishPile_Small_1a.SM_RubbishPile_Small_1a" :`1` "/Game/Assets/Meshes/SM_RubbishPile_Medium_1a.SM_RubbishPile_Medium_1a" :`2` "/Game/Assets/Meshes/SM_RubbishPile_Large_1a.SM_RubbishPile_Large_1a" :!type "StaticMesh Object Reference") :!label _label)
    (bind _output_get (set `self.SpringArmNewLength` (select `int` _meshsize :`0` 300.0 :`1` 500.0 :`2` 800.0 :!type "Float (single-precision)")))
    (bind (_direction _alpha) (`Timeline|SpringArmLength` :!via `PlayFromStart`)
      (:`Update`
        (set `SpringArmComponent.TargetArmLength` (`KismetMathLibrary.Lerp` (`SpringArmComponent.TargetArmLength` _springarm) _output_get _alpha) _springarm)))
    (elif (<= _pendingscore (`self.MediumMeshValue`))
      (set `self.MeshSize` 1)
      (goto _label)
      (elif (>= _pendingscore (`self.LargeMeshValue`))
        (set `self.MeshSize` 2)
        (goto _label)))))

(fn `Buoyancy`
  (returns (OutDistance :type "Float (double-precision)"))
  (bind _outhit (`KismetSystemLibrary.LineTraceSingleForObjects` :`Start` (`SceneComponent.K2_GetComponentLocation` (`self.CapsuleComponent`)) :`End` (0.0 0.0 -5000.0) :`ObjectTypes` (`|MakeArray` "ObjectTypeQuery1" :!type "EObjectTypeQuery Enum") :`DrawDebugType` "ForDuration" :`DrawTime` 1.0))
  (bind _outhit_2 (`KismetSystemLibrary.LineTraceSingleForObjects` :`Start` (`.ImpactPoint` (`GameplayStatics.BreakHitResult` _outhit)) :`End` (0.0 0.0 5000.0) :`ObjectTypes` (`|MakeArray` "ObjectTypeQuery2" :!type "EObjectTypeQuery Enum") :`DrawDebugType` "ForDuration" :`DrawTime` 1.0))
  (return (`.Distance` (`GameplayStatics.BreakHitResult` _outhit_2))))

(fn `RemoveTime`
  (bind _gmref (`self.GMRef`))
  (bind _returnvalue (- (`/Game/Blueprints/Character/GM_Default.Seconds` _gmref) 10))
  (`self.Damage`)
  (if (<= _returnvalue 0)
    (set `/Game/Blueprints/Character/GM_Default.Minutes` (- (`/Game/Blueprints/Character/GM_Default.Minutes` _gmref) 1) _gmref)
    (set `/Game/Blueprints/Character/GM_Default.Seconds` (+ _returnvalue 59) _gmref)
    (else
      (set `/Game/Blueprints/Character/GM_Default.Seconds` _returnvalue _gmref))))

(fn `UserConstructionScript`)