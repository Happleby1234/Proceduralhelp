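; Player slime character that moves, looks, creates the HUD and absorbs BP_Trash actors on capsule overlap.
; Overlapped trash is briefly attached, its mesh geometry appended to shared arrays to build procedural mesh sections, then destroyed.
; The game mode's TrashCollected event, bound on Tick, swaps the slime between three rubbish-pile meshes by PendingScore and eases spring arm length through a timeline.
; Trace-based buoyancy and bobbing logic exist but are unconnected.
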(event `self.ReceiveBeginPlay`
  (`|ExecutionSequence`
    (:`then_0`
      (bind _asgm_default (cast `/Game/Blueprints/Character/GM_Default` (`GameplayStatics.GetGameMode`)))
      (set `self.GMRef` _asgm_default))
    (:`then_1`
      (bind _returnvalue (`|CreateWidget` "/Game/Blueprints/Widgets/UI/WBP_HUD.WBP_HUD_C" (`GameplayStatics.GetPlayerController` 0)))
      (bind _output_get (set `self.HUDRef` _returnvalue))
      (`UserWidget.AddToViewport` _output_get 0))))

(event `InputAxis|MoveForward`
  (params (AxisValue :type "Float (single-precision)"))
  ;[1 0.02344 0] Movement
  (`self.AddMovementInput` (`self.GetActorForwardVector`) AxisValue))

(event `InputAxis|LookUp`
  (params (AxisValue :type "Float (single-precision)"))
  ;[1 0.02344 0] Movement
  (`self.AddControllerPitchInput` AxisValue))

(event `InputAxis|LookRight`
  (params (AxisValue :type "Float (single-precision)"))
  ;[1 0.02344 0] Movement
  (`self.AddControllerYawInput` AxisValue))

(event `InputAxis|MoveRight`
  (params (AxisValue :type "Float (single-precision)"))
  ;[1 0.02344 0] Movement
  (`self.AddMovementInput` (`self.GetActorRightVector`) AxisValue))

(event `self.ReceiveTick`
  (params (DeltaSeconds :type "Float (single-precision)"))
  (add `/Game/Blueprints/Character/GM_Default.TrashCollected` (`self.GMRef`) (delegate `MeshChange`)))

(event `MeshChange`
  (bind _springarm (`self.SpringArm`))
  (bind _meshsize (`self.MeshSize`))
  (bind _pendingscore (`/Game/Blueprints/Character/GM_Default.PendingScore` (`self.GMRef`)))
  (if (<= _pendingscore (`self.SmallMeshValue`))
    (set `self.MeshSize` 0)
    (`StaticMeshComponent.SetStaticMesh` (`self.SlimeMesh`) (select `int` _meshsize :`0` "/Game/Assets/Meshes/SM_RubbishPile_Small_1a.SM_RubbishPile_Small_1a" :`1` "/Game/Assets/Meshes/SM_RubbishPile_Medium_1a.SM_RubbishPile_Medium_1a" :`2` "/Game/Assets/Meshes/SM_RubbishPile_Large_1a.SM_RubbishPile_Large_1a" :!type "StaticMesh Object Reference") :!label _label)
    (bind _output_get (set `self.SpringArmNewLength` (select `int` _meshsize :`0` 300.0 :`1` 500.0 :`2` 800.0 :!type "Float (single-precision)")))
    (bind (_direction _alpha) (`Timeline|SpringArmLength` :!via `PlayFromStart`)
      (:`Update`
        (set `SpringArmComponent.TargetArmLength` (`KismetMathLibrary.Lerp` (`SpringArmComponent.TargetArmLength` _springarm) _output_get _alpha) _springarm)))
    (elif (<= _pendingscore (`self.MediumMeshValue`))
      (set `self.MeshSize` 1)
      (goto _label)
      (elif (>= _pendingscore (`self.LargeMeshValue`))
        (set `self.MeshSize` 2)
        (goto _label)))))

(event `self.Capsule.OnComponentBeginOverlap`
  (params (OverlappedComponent :type "PrimitiveComponent Object Reference") (OtherActor :type "Actor Object Reference") (OtherComp :type "PrimitiveComponent Object Reference") (OtherBodyIndex :type Integer) (bFromSweep :type Boolean) (SweepResult :type "HitResult Structure (by ref)"))
  (bind _attachedactorarray (`self.AttachedActorArray`))
  (bind _returnvalue (`KismetArrayLibrary.Array_LastIndex` _attachedactorarray))
  (bind _asbp_trash (cast `/Game/Blueprints/TrashObjects/BP_Trash` OtherActor))
  (`|ExecutionSequence`
    (:`then_0`
      (bind _output_get (set `self.TrashRef` _asbp_trash))
      (`self.K2_AttachToComponent` _output_get (`self.SlimeMesh`) "None" "KeepWorld" "KeepWorld" "KeepWorld" true)
      (`KismetArrayLibrary.Array_Add` _attachedactorarray _output_get)
      (`|ExecutionSequence`
        (:`then_0`
          (bind (_vertices _triangles _normals _uvs _tangents) (`KismetProceduralMeshLibrary.GetSectionFromStaticMesh` (`StaticMeshComponent.StaticMesh` (`/Game/Blueprints/TrashObjects/BP_Trash.TrashMesh` (`|GetArrayItem` _attachedactorarray _returnvalue))) 0 _returnvalue))
          (`|ExecutionSequence`
            (:`then_0`
              (`KismetArrayLibrary.Array_Append` (`self.BB_Vertices`) _vertices))
            (:`then_1`
              (`KismetArrayLibrary.Array_Append` (`self.BB_Triangles`) _triangles))
            (:`then_2`
              (`KismetArrayLibrary.Array_Append` (`self.BB_Normals`) _normals))
            (:`then_3`
              (`KismetArrayLibrary.Array_Append` (`self.BB_Tangents`) _tangents))
            (:`then_5`
              (`self.K2_DestroyActor` _output_get))))))
    (:`then_1`
      (`ProceduralMeshComponent.CreateMeshSection_LinearColor` :`self` (`self.ProceduralMesh`) :`SectionIndex` _returnvalue :`Vertices` (`self.BB_Vertices`) :`Triangles` (`self.BB_Triangles`) :`Normals` (`self.BB_Normals`) :`Tangents` (`self.BB_Tangents`) :`bCreateCollision` true))))

(fn `Buoyancy`
  (returns (OutDistance :type "Float (double-precision)"))
  (bind _outhit (`KismetSystemLibrary.LineTraceSingleForObjects` :`Start` (`SceneComponent.K2_GetComponentLocation` (`self.CapsuleComponent`)) :`End` (0.0 0.0 -5000.0) :`ObjectTypes` (`|MakeArray` "ObjectTypeQuery1" :!type "EObjectTypeQuery Enum") :`DrawDebugType` "ForDuration" :`DrawTime` 1.0))
  (bind _outhit_2 (`KismetSystemLibrary.LineTraceSingleForObjects` :`Start` (`.ImpactPoint` (`GameplayStatics.BreakHitResult` _outhit)) :`End` (0.0 0.0 5000.0) :`ObjectTypes` (`|MakeArray` "ObjectTypeQuery2" :!type "EObjectTypeQuery Enum") :`DrawDebugType` "ForDuration" :`DrawTime` 1.0))
  (return (`.Distance` (`GameplayStatics.BreakHitResult` _outhit_2))))

(fn `UserConstructionScript`)