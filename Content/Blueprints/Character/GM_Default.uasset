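; Game mode for a timed trash-collection game, ending when the last tagged trash is picked up or time runs out.
; A looping one-second timer event drives the minute/second countdown.
; Collected trash adds to a pending score and grants bonus time, a separate function banks it into the total, and both fire TrashCollected.
; GameEnds swaps the player HUD for an end screen with remaining time and switches to UI-only input.
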(event `self.ReceiveBeginPlay`
  ;[0 1 0.5547 0.5] BeginPlay
  (bind _returnvalue (`GameplayStatics.GetActorOfClass` "/Game/Blueprints/SetObjects/BP_WaterPlane.BP_WaterPlane_C"))
  (set `self.WaterRef` _returnvalue)
  (`WidgetBlueprintLibrary.SetInputMode_GameOnly` (`GameplayStatics.GetPlayerController` 0))
  (`KismetSystemLibrary.K2_SetTimerDelegate` (delegate `Timer`) 1.0 true)
  (bind _asbp_character (cast `/Game/Blueprints/Character/BP_Character` (`GameplayStatics.GetPlayerCharacter` 0)))
  (set `self.PlayerRef` _asbp_character))

(event `/Game/Blueprints/TrashObjects/BPI_TrashCollected.TrashPickedUp`
  ;[0 1 0.25 0.5] TrashPickedUpInterface
  (bind _outactors (`GameplayStatics.GetAllActorsOfClassWithTag` "/Game/Blueprints/TrashObjects/BP_Trash.BP_Trash_C" "Trash"))
  (if (<= (`KismetArrayLibrary.Array_Length` _outactors) 1)
    (`self.GameEnds` (`self.Minutes`) (`self.Seconds`))))

(event `Timer`
  (if (`self.TimerActive`)
    ;[1 0.07031 0 0.5] Timer
    (`|ExecutionSequence`
      (:`then_0`
        ;;[0.9219 0 1 0.5] Out Of Time
        (if (== (`self.Minutes`) 0)
          (set `self.MinutesOut` true)
          (set `self.RemainingMinutes` 0)
          (if (== (`self.Seconds`) 0)
            (set `self.SecondsOut` true)
            (set `self.RemainingSeconds` 0))))
      (:`then_1`
        (set `self.Seconds` (- (`self.Seconds`) 1))
        (if (< (`self.Seconds`) 0)
          (if (and (`self.SecondsOut`) (`self.MinutesOut`))
            ;;[0.125 1 0 0.5] If Time Runs Out
            (`self.GameEnds` (`self.RemainingMinutes`) (`self.RemainingSeconds`))
            (set `self.TimerActive` false)
            (else
              (set `self.Minutes` (- (`self.Minutes`) 1))
              (set `self.Seconds` 59))))))))

(fn `AddBonusTime`
  (bind _returnvalue (+ (`self.Seconds`) (`self.BonusTime`)))
  (if (<= _returnvalue 60)
    (set `self.Seconds` _returnvalue)
    (else
      (set `self.Minutes` (+ (`self.Minutes`) 1))
      (set `self.Seconds` (- _returnvalue 60)))))

(fn `AddToPendingScore`
  (params (TrashReference :type "/Game/Blueprints/TrashObjects/BP_Trash Object Reference"))
  (bind _output_get (set `self.PendingScore` (+ (`self.PendingScore`) (`/Game/Blueprints/TrashObjects/BP_Trash.TrashValue` TrashReference))))
  (`self.AddBonusTime`)
  (`self.TrashCollected`)
  (`KismetSystemLibrary.PrintString` (`KismetStringLibrary.Concat_StrStr` "Pending Score" ": " (`KismetStringLibrary.Conv_IntToString` _output_get))))

(fn `AddToTotalScore`
  (bind _output_get (set `self.CurrentScore` (+ (`self.CurrentScore`) (`self.PendingScore`))))
  (set `self.PendingScore` 0)
  (`self.TrashCollected`)
  (`KismetSystemLibrary.PrintString` (`KismetStringLibrary.Concat_StrStr` "Current Score" ": " (`KismetStringLibrary.Conv_IntToString` _output_get))))

(fn `GameEnds`
  (params (RemainingMinutes :type Integer) (RemainingSeconds :type Integer))
  (bind _returnvalue (`GameplayStatics.GetPlayerController` 0))
  (set `self.RemainingMinutes` RemainingMinutes)
  (set `self.RemainingSeconds` RemainingSeconds)
  (`Widget.RemoveFromParent` (`/Game/Blueprints/Character/BP_Character.HUDRef` (`self.PlayerRef`)))
  (bind _returnvalue_2 (`|CreateWidget` "/Game/Blueprints/Widgets/EndScreen/WBP_EndScreen.WBP_EndScreen_C" _returnvalue RemainingSeconds RemainingMinutes))
  (`UserWidget.AddToViewport` _returnvalue_2 0)
  (`self.DisableInput` _returnvalue)
  (`WidgetBlueprintLibrary.SetInputMode_UIOnlyEx` _returnvalue _returnvalue_2)
  (set `PlayerController.bShowMouseCursor` true _returnvalue))

(fn `UserConstructionScript`)