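; BPC_Buoyancy is a component Blueprint named for buoyancy that holds only debug printing and a test trace, with no buoyancy forces.
; Init prints the owner's display name and whether the ParentsCollision reference is valid.
; Tick line-traces against ParentsCollision alone, from its world location straight up along Z, with the trace drawn for debugging.
; The trace result is unused, and ParentsCollision is not assigned in this graph.
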(event `Init`
  (`KismetSystemLibrary.PrintString` (`KismetSystemLibrary.GetDisplayName` (`self.GetOwner`)))
  (`KismetSystemLibrary.PrintString` (`KismetStringLibrary.Conv_BoolToString` (`KismetSystemLibrary.IsValid` (`self.parents collision`)))))

(event `self.ReceiveTick`
  (params (DeltaSeconds :type "Float (single-precision)"))
  (bind _parents_collision (`self.parents collision`))
  (bind _returnvalue (`SceneComponent.K2_GetComponentLocation` _parents_collision))
  (`PrimitiveComponent.K2_LineTraceComponent` _parents_collision _returnvalue (+ _returnvalue (0.0 0.0 5000.0)) true true false))