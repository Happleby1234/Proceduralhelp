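; BP_WaterPlane is a water surface actor that computes Gerstner wave height at a given world XY position.
; GetWaveHeight sums four Gertsner samples in differing directions, two at full scale and two at half wavelength, amplitude and time, and returns the Z displacement.
; WaveTime drives the phase but is not advanced here, as Tick is empty.
; BeginPlay only caches the player's BP_Character.
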(event `self.ReceiveBeginPlay`
  (bind _asbp_character (cast `/Game/Blueprints/Character/BP_Character` (`GameplayStatics.GetPlayerCharacter` 0)))
  (set `self.PlayerRef` _asbp_character))

(event `self.ReceiveTick`
  (params (DeltaSeconds :type "Float (single-precision)")))

(fn `Gertsner`
  (params (WorldPosition :type "Vector Structure") (Direction :type "Vector Structure") (WaveRotation :type "Float (double-precision)") (`WaveLength ` :type "Float (double-precision)") (WaveAmplitude :type "Float (double-precision)") (WaveSteepness :type "Float (double-precision)") (Speed :type "Float (double-precision)"))
  (returns (Displacement :type "Vector Structure"))
  (bind _returnvalue (`KismetMathLibrary.Normal` (`KismetMathLibrary.RotateAngleAxis` Direction (`KismetMathLibrary.MapRangeUnclamped` WaveRotation 0.0 1.0 0.0 360.0))))
  (bind _returnvalue_2 (/ (+ (* (`KismetMathLibrary.Dot_VectorVector` (`KismetMathLibrary.MakeVector` (.x WorldPosition) (.y WorldPosition)) _returnvalue) (/ (`KismetMathLibrary.MultiplyByPi` 2.0) `WaveLength `)) Speed) (`KismetMathLibrary.MultiplyByPi` 2.0)))
  (bind _returnvalue_3 (* (* (`KismetMathLibrary.Cos` _returnvalue_2) WaveSteepness) WaveAmplitude))
  (return (`KismetMathLibrary.MakeVector` (* (.x _returnvalue) _returnvalue_3) (* (.y _returnvalue) _returnvalue_3) (* (`KismetMathLibrary.Sin` _returnvalue_2) WaveAmplitude))))

(fn `GetWaveHeight`
  (params (X :type "Float (double-precision)") (Y :type "Float (double-precision)"))
  (returns (WaveHeight :type "Float (double-precision)"))
  (bind _wavelength (`self.WaveLength`))
  (bind _waveamplitude (`self.WaveAmplitude`))
  (bind _wavesteepness (`self.WaveSteepness`))
  (bind _wavetime (`self.WaveTime`))
  (bind _z (.z (`self.K2_GetActorLocation`)))
  (bind _returnvalue (* _wavelength 0.5))
  (bind _returnvalue_2 (* _wavetime 0.5))
  (bind _returnvalue_3 (* _waveamplitude 0.5))
  (bind _returnvalue_4 (`KismetMathLibrary.MakeVector` X Y _z))
  (bind (_returnvalue_x _returnvalue_y _returnvalue_z) (`KismetMathLibrary.BreakVector` (+ (+ (`self.Gertsner` _returnvalue_4 (`KismetMathLibrary.MakeVector` 1.0 1.0 _z) 1.0 _wavelength _waveamplitude _wavesteepness _wavetime) (`self.Gertsner` _returnvalue_4 (`KismetMathLibrary.MakeVector` 1.0 0.5 _z) 1.0 _wavelength _waveamplitude _wavesteepness _wavetime)) (+ (`self.Gertsner` _returnvalue_4 (`KismetMathLibrary.MakeVector` 0.0 1.0 _z) 1.0 _returnvalue _returnvalue_3 _wavesteepness _returnvalue_2) (`self.Gertsner` _returnvalue_4 (`KismetMathLibrary.MakeVector` 1.0 0.0 _z) 1.0 _returnvalue _returnvalue_3 _wavesteepness _returnvalue_2)))))
  (return _returnvalue_z))

(fn `UserConstructionScript`)