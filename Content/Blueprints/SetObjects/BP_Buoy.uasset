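; BP_Buoy is a set-object buoy that fakes floating motion with a timeline started on BeginPlay.
; Each BuoyancyFake update rocks pitch and roll by a few degrees, keeps yaw, and adds a small alpha-scaled Z offset to the current location, so height accumulates.
; Unconnected leftover nodes would set height from the game mode water's GetWaveHeight, but never run.
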(event `self.ReceiveBeginPlay`
  (bind _returnvalue (`self.K2_GetActorLocation`))
  (bind (_returnvalue_roll _returnvalue_pitch _returnvalue_yaw) (`KismetMathLibrary.BreakRotator` (`self.K2_GetActorRotation`)))
  (bind (_direction _alpha) (`Timeline|BuoyancyFake`)
    (:`Update`
      (`self.K2_SetActorLocationAndRotation` (`KismetMathLibrary.VLerp` _returnvalue (+ _returnvalue (0.0 0.0 0.25)) _alpha) (`KismetMathLibrary.RLerp` (`KismetMathLibrary.MakeRotator` -2.0 -2.0 _returnvalue_yaw) (`KismetMathLibrary.MakeRotator` 2.0 2.0 _returnvalue_yaw) _alpha)))))

(event `self.ReceiveTick`
  (params (DeltaSeconds :type "Float (single-precision)")))

(fn `UserConstructionScript`)