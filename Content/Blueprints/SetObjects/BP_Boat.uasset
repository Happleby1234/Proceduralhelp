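; BP_Boat is an AI-driven boat pawn that wanders the level and takes time away from BP_Character when it hits the player.
; A looping timer sends it to random points within the NavMesh bounds, pausing during each move and resuming only on success.
; A second timer restarts a timeline that eases the mesh toward its velocity direction with a yaw offset.
; Hit penalties are throttled by a resetting DoOnce.
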(event `Rotation`
  (bind _boatmesh (`self.BoatMesh`))
  (bind (_returnvalue_roll _returnvalue_pitch _returnvalue_yaw) (`KismetMathLibrary.BreakRotator` (`KismetMathLibrary.Conv_VectorToRotator` (`MovementComponent.Velocity` (`self.FloatingPawnMovement`)))))
  (bind (_direction _alpha) (`Timeline|Alpha` :!via `PlayFromStart`)
    (:`Update`
      (`SceneComponent.K2_SetRelativeRotation` _boatmesh (`KismetMathLibrary.RLerp` (`KismetMathLibrary.Conv_VectorToRotator` (`SceneComponent.GetForwardVector` _boatmesh)) (`KismetMathLibrary.MakeRotator` _returnvalue_roll _returnvalue_pitch (- _returnvalue_yaw 90.0)) _alpha true) false false))))

(event `self.ReceiveBeginPlay`
  (bind _returnvalue (`KismetSystemLibrary.K2_SetTimerDelegate` (delegate `AI MoveTo`) 1.0 true))
  (`KismetSystemLibrary.K2_SetTimerDelegate` (delegate `Rotation`) 1.0 true))

(event `AI MoveTo`
  (bind (_origin _boxextent) (`KismetSystemLibrary.GetComponentBounds` (`Brush.BrushComponent` (`self.NavMesh`))))
  (`|AIMoveTo` self (`KismetMathLibrary.RandomPointInBoundingBox` _origin _boxextent) null 0.1
    (:`then`
      (`KismetSystemLibrary.K2_PauseTimerHandle` (stale `self.ReceiveBeginPlay` _returnvalue)))
    (:`OnSuccess`
      (`KismetSystemLibrary.K2_UnPauseTimerHandle` (stale `self.ReceiveBeginPlay` _returnvalue)))))

(event `self.BoatMesh.OnComponentHit`
  (params (HitComponent :type "PrimitiveComponent Object Reference") (OtherActor :type "Actor Object Reference") (OtherComp :type "PrimitiveComponent Object Reference") (NormalImpulse :type "Vector Structure") (Hit :type "HitResult Structure (by ref)"))
  (bind _asbp_character (cast `/Game/Blueprints/Character/BP_Character` OtherActor))
  (`/Engine/EditorBlueprintResources/StandardMacros.DoOnce` false :!label _label
    (:`Completed`
      (`/Game/Blueprints/Character/BP_Character.RemoveTime` _asbp_character)
      (`KismetSystemLibrary.Delay` 1.0)
      (goto _label :!via `Reset`))))

(fn `UserConstructionScript`)