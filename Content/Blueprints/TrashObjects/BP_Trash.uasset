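; BP_Trash is a trash actor with a random value of 1 to 5, appearing as a bin bag or plastic bottle.
; The construction script randomly picks mesh and material through a pure random node, so the two can mismatch.
; BeginPlay caches GM_Default and plays a timeline that rocks the actor and nudges it upward from its current location.
; The overlap handler only casts to BP_Trash; a separate event logs and destroys the actor.
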(event `self.Sphere.OnComponentBeginOverlap`
  (params (OverlappedComponent :type "PrimitiveComponent Object Reference") (OtherActor :type "Actor Object Reference") (OtherComp :type "PrimitiveComponent Object Reference") (OtherBodyIndex :type Integer) (bFromSweep :type Boolean) (SweepResult :type "HitResult Structure (by ref)"))
  ;[0.2188 0 1] PickupEvent
  (cast `/Game/Blueprints/TrashObjects/BP_Trash` OtherActor))

(event `self.ReceiveBeginPlay`
  (bind _returnvalue (`self.K2_GetActorLocation`))
  (bind (_returnvalue_roll _returnvalue_pitch _returnvalue_yaw) (`KismetMathLibrary.BreakRotator` (`self.K2_GetActorRotation`)))
  ;[0.5703 0 1] BeginPlay
  (`|ExecutionSequence`
    (:`then_0`
      ;;[0 1 0.01562] GameModeReference
      (bind _asgm_default (cast `/Game/Blueprints/Character/GM_Default` (`GameplayStatics.GetGameMode`)))
      (set `self.GMRef` _asgm_default)
      (set `self.TrashValue` (`KismetMathLibrary.RandomIntegerInRange` 1 5)))
    (:`then_1`
      (bind (_direction _alpha) (`Timeline|BobbingAnim`)
        (:`Update`
          (`self.K2_SetActorLocationAndRotation` (`KismetMathLibrary.VLerp` _returnvalue (+ _returnvalue (0.0 0.0 0.1)) _alpha) (`KismetMathLibrary.RLerp` (`KismetMathLibrary.MakeRotator` -2.0 -2.0 _returnvalue_yaw) (`KismetMathLibrary.MakeRotator` 2.0 2.0 _returnvalue_yaw) _alpha)))))))

(event `DestroyActor`
  (`KismetSystemLibrary.PrintString` "ActorDestroyed")
  (`self.K2_DestroyActor`))

(fn `UserConstructionScript`
  (bind _trashmesh (`self.TrashMesh`))
  (bind _returnvalue (select `int` (`KismetMathLibrary.RandomIntegerInRange` 0 1) :`0` "/Game/Assets/Meshes/SM_BinBag_zAxis.SM_BinBag_zAxis" :`1` "/Game/Assets/Meshes/SM_PlasticBottle_1c.SM_PlasticBottle_1c" :!type "StaticMesh Object Reference"))
  (`StaticMeshComponent.SetStaticMesh` _trashmesh _returnvalue)
  (`PrimitiveComponent.SetMaterial` _trashmesh 0 (`StaticMesh.GetMaterial` _returnvalue 0)))