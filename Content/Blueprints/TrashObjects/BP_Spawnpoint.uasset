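; Spawn point actor that scatters BP_Trash across the floor within its Spawnbounds box when play begins.
; BeginPlay calls Spawntrash in a loop driven by AmountofTrash.
; Each call picks random coordinates in the box, line-traces downward against WorldStatic objects from above, and spawns trash at the hit location without checking for a hit.
; Each trash receives a reference to its spawn point and is added to TrashinLevel.
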(event `self.ReceiveBeginPlay`
  (for _ (range (+ (`self.AmountofTrash`) 1))
    (`self.Spawntrash`)))

(fn `Spawntrash`
  (bind (_origin _boxextent) (`KismetSystemLibrary.GetComponentBounds` (`self.Spawnbounds`)))
  (bind _returnvalue (`KismetMathLibrary.MakeVector` (.x (`KismetMathLibrary.RandomPointInBoundingBox` _origin _boxextent)) (.y (`KismetMathLibrary.RandomPointInBoundingBox` _origin _boxextent)) (+ (.z (`KismetMathLibrary.RandomPointInBoundingBox` _origin _boxextent)) 2500.0)))
  ;[1 1 1] finding the floor to spawn on combined with the area found inside the box
  (bind _outhit (`KismetSystemLibrary.LineTraceSingleForObjects` :`Start` _returnvalue :`End` (+ _returnvalue (* (* (`self.GetActorUpVector`) -1) 5000.0)) :`ObjectTypes` (`|MakeArray` "ObjectTypeQuery1" :!type "EObjectTypeQuery Enum") :`DrawDebugType` "ForDuration"))
  ;[1 1 1] spawning the actor
  (bind _returnvalue_2 (`|SpawnActorFromClass` "/Game/Blueprints/TrashObjects/BP_Trash.BP_Trash_C" (`KismetMathLibrary.MakeTransform` (`KismetMathLibrary.MakeVector` (.x (`.Location` (`GameplayStatics.BreakHitResult` _outhit))) (.y (`.Location` (`GameplayStatics.BreakHitResult` _outhit))) (+ (.z (`.Location` (`GameplayStatics.BreakHitResult` _outhit))) 0.0)) (`KismetMathLibrary.MakeRotator` 0.0 0.0 (`KismetMathLibrary.RandomFloat`))) "AdjustIfPossibleButAlwaysSpawn" "OverrideRootScale" null (0.0 0.0 0.0) 0 null))
  (set `/Game/Blueprints/TrashObjects/BP_Trash.SpawnpointRef` self _returnvalue_2)
  (`KismetArrayLibrary.Array_Add` (`self.TrashinLevel`) _returnvalue_2))

(fn `UserConstructionScript`)